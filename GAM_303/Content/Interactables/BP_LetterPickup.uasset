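; BP_LetterPickup is an interactable physics pickup, a letter by its name, that the player can carry and drop.
; Through interact and drop events, it attaches its Cube to the player's Arrow1 with physics and collision off, provided the player holds nothing.
; Dropping detaches the actor and restores collision and physics, but leaves the player's IsHolding flag untouched.
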(event `self.INT_Interact`
  (params (PlayerRef :type "/Game/Player/BP_PlayerChar Object Reference"))
  (bind _cube (`self.Cube`))
  ; Pick up Item
  (if (not (`/Game/Player/BP_PlayerChar.IsHolding?` PlayerRef))
    (set `/Game/Player/BP_PlayerChar.IsHolding?` true PlayerRef)
    (`PrimitiveComponent.SetSimulatePhysics` _cube false)
    (`PrimitiveComponent.SetCollisionEnabled` _cube "NoCollision")
    (`SceneComponent.K2_AttachToComponent` (`self.Cube`) (`/Game/Player/BP_PlayerChar.Arrow1` PlayerRef) "None" "SnapToTarget" "SnapToTarget" "KeepWorld" false)))

(event `self.INT_Drop`
  (bind _cube (`self.Cube`))
  ; Drop Item
  (`self.K2_DetachFromActor` "KeepWorld" "KeepWorld" "KeepWorld")
  (`PrimitiveComponent.SetCollisionEnabled` _cube "QueryAndPhysics")
  (`PrimitiveComponent.SetSimulatePhysics` _cube true))

(fn `UserConstructionScript`)